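; Player-piloted Predator Missile killstreak that takes possession of the controller and drops from high above the map.
; Mouse axes apply steering forces, with transforms copied to remotes, and left click gives a one-time downward boost.
; A per-tick camera trace detects impact, then a sphere trace plus line-of-sight check damages characters on "head" bone hits through the game mode.
; Control then returns to the original player and the missile is destroyed.
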(event Custom|AddForceForwardAll
  (params (Target :type Primitive%20Component%20Object%20Reference) (Force :type Vector) (NewTransform :type Transform%20%28by%20ref%29))
  ;[1 1 1] Move
  (Networking|SwitchHasAuthority
    (:Remote
      (Transformation|SetWorldTransform Target NewTransform false false))))

(event Custom|Possess
  ;[1 1 1] Possess
  (Pawn|Possess (Variables|Default|GetNewPlayerController) self))

(event Custom|Boost
  ;[1 1 1] Add Force
  (Utilities|FlowControl|DoOnce false
    (:Completed
      (Physics|AddForce (Variables|Default|GetMissile) "0, 0,-1000000.000000" "None" true))))

(event Custom|HitDetectionServer
  (bind _camera (Variables|Default|GetCamera))
  (bind _missile (Variables|Default|GetMissile))
  (bind _returnvalue (Transformation|GetWorldLocation _camera))
  (bind _returnvalue_2 (Transformation|GetWorldLocation _missile))
  ;[1 1 1] Hit
  (bind _returnvalue_3 (Collision|LineTraceByChannel _returnvalue (+ _returnvalue (* (Math|Vector|GetForwardVector _camera) 2e+02)) "TraceTypeQuery1" true 0 "ForDuration" true "(R=1.000000,G=0.000000,B=0.000000,A=1.000000)" "(R=0.000000,G=1.000000,B=0.000000,A=1.000000)" 3.0))
  (if _returnvalue_3
    (Utilities|FlowControl|DoOnce false
      (:Completed
        (bind (_outhits _returnvalue_4) (Collision|MultiSphereTraceByChannel _returnvalue_2 _returnvalue_2 1.5e+03 "TraceTypeQuery3" true 0 "ForDuration"))
        (if _returnvalue_4
          (Pawn|Possess (Variables|Default|GetNewPlayerController) (Variables|Default|GetOriginalPlayer))
          (for _array_element _outhits
            (bind _asfirst_person_character (Utilities|Casting|CastToFirstPersonCharacter (.HitActor (Collision|BreakHitResult _array_element))))
            (bind _outhit (Collision|LineTraceByChannel _returnvalue_2 (Transformation|GetActorLocation _asfirst_person_character) "TraceTypeQuery3" true 0 "ForDuration"))
            (Utilities|Casting|CastToFirstPersonCharacter (.HitActor (Collision|BreakHitResult _outhit)))
            (if (Utilities|Name|Equal(Name) (.HitBoneName (Collision|BreakHitResult _array_element)) "head")
              (bind _asnew_player_state (Utilities|Casting|CastToNewPlayerState (Variables|/Script/Engine.Pawn|GetPlayerState _asfirst_person_character)))
              (bind _asnew_player_state_2 (Utilities|Casting|CastToNewPlayerState (Variables|/Script/Engine.Controller|GetPlayerState (Variables|Default|GetNewPlayerController))))
              (bind _asfirst_person_gamemode (Utilities|Casting|CastToFirstPersonGamemode (Game|GetGameMode)))
              (Default|DamageandCheckifPlayerDead _asfirst_person_gamemode _asfirst_person_character _asnew_player_state_2 _asnew_player_state (* (Math|Vector|MakeVector (.X (Math|Vector|BreakVector (- (.TraceEnd (Collision|BreakHitResult _outhit)) (.TraceStart (Collision|BreakHitResult _outhit))))) (.Y (Math|Vector|BreakVector (- (.TraceEnd (Collision|BreakHitResult _outhit)) (.TraceStart (Collision|BreakHitResult _outhit))))) (+ (.Z (Math|Vector|BreakVector (- (.TraceEnd (Collision|BreakHitResult _outhit)) (.TraceStart (Collision|BreakHitResult _outhit))))) 4e+02)) 3.5e+02) (.Location (Collision|BreakHitResult _outhit)) 0 (== _asfirst_person_character (Variables|Default|GetOriginalPlayer)) true 1e+02)
              (Actor|DestroyActor)))
          (Pawn|Possess (Variables|Default|GetNewPlayerController) (Variables|Default|GetOriginalPlayer))
          (Actor|DestroyActor)
          (else
            (Pawn|Possess (Variables|Default|GetNewPlayerController) (Variables|Default|GetOriginalPlayer))
            (Actor|DestroyActor)))))))

(event Custom|AddForceForwardServer
  (params (Target :type Primitive%20Component%20Object%20Reference) (Force :type Vector))
  ;[1 1 1] Move
  (Physics|AddForce Target Force "None" true)
  (CallFunction|AddForceForwardAll Target "0, 0, 0" (Transformation|GetWorldTransform Target)))

(event Custom|AddForceRightServer
  (params (Target :type Primitive%20Component%20Object%20Reference) (Force :type Vector))
  ;[1 1 1] Move
  (Physics|AddForce Target Force "None" true)
  (CallFunction|AddForceRightAll Target "0, 0, 0" (Transformation|GetWorldTransform Target)))

(event Custom|AddForceRightAll
  (params (Target :type Primitive%20Component%20Object%20Reference) (Force :type Vector) (NewTransform :type Transform%20%28by%20ref%29))
  ;[1 1 1] Move
  (Networking|SwitchHasAuthority
    (:Remote
      (Transformation|SetWorldTransform Target NewTransform false false))))

(event EventBeginPlay
  ;[1 1 1] Add Force
  (Transformation|SetWorldTransform (Variables|Default|GetMissile) (Math|Transform|MakeTransform "0, 0,30000.000000") false false)
  (Physics|AddForce (Variables|Default|GetMissile) "0.000000, 0,-100000.000000" "None" true)
  (CallFunction|Possess))

(event EventTick
  (params (DeltaSeconds :type Float%20%28single-precision%29))
  ;[1 1 1] Hit
  (CallFunction|HitDetectionServer))

(event Input|MouseEvents|MouseX
  (params (AxisValue :type Float%20%28single-precision%29))
  ;[1 1 1] Move
  (CallFunction|AddForceRightServer (Variables|Default|GetMissile) (* (* (Math|Vector|GetRightVector (Variables|Default|GetCamera)) 5e+03) AxisValue)))

(event Input|MouseEvents|MouseY
  (params (AxisValue :type Float%20%28single-precision%29))
  ;[1 1 1] Move
  (CallFunction|AddForceForwardServer (Variables|Default|GetMissile) (* (* (Math|Vector|GetUpVector (Variables|Default|GetCamera)) 5e+03) AxisValue)))

(event Input|MouseEvents|LeftMouseButton
  (params (Key :type Key%20Structure))
  ;[1 1 1] Add Force
  (:Pressed
    (CallFunction|Boost)))

(fn ConstructionScript)