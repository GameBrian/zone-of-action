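; Player state for a multiplayer first-person shooter, holding the player's create-a-class loadout and selected killstreaks.
; It loads both from a save slot on BeginPlay and writes them back through a SaveGame object when the class is saved.
; Events edit the killstreak selection, show a hitmarker widget for a locally controlled target, and ask the game mode to spawn the player with the saved class.
; OnRep handlers for team, killstreak and health are empty.
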(event Custom|Hitmarker
  (params (Target :type Pawn%20Object%20Reference))
  (if (Pawn|IsLocallyControlled Target)
    (bind _returnvalue (UserInterface|CreateWidget "/Game/UMG/Hitmarker.Hitmarker_C"))
    (UserInterface|Viewport|AddtoViewport _returnvalue 0)))

(event Custom|Selected%20Killstreaks
  (params (AddOrSubtract :type Boolean) (Killstreak :type Killstreak%20Base%20Class%20Reference) (Playerstate :type New%20Player%20State%20Object%20Reference))
  (if AddOrSubtract
    (Utilities|Array|Add (Variables|NewPlayerState_C|GetSelectedKillstreaks Playerstate) Killstreak)
    (else
      (Utilities|Array|RemoveItem (Variables|NewPlayerState_C|GetSelectedKillstreaks Playerstate) Killstreak))))

(event Custom|SetGUI
  (params (GUI :type Ingame%20GUI%20Object%20Reference))
  (Variables|Default|SetGUI GUI))

(event Custom|SaveCreateAClass
  (CallFunction|SavePlayerInfo (Variables|Default|GetCreateAClass) (Variables|Default|GetSelectedKillstreaks)))

(event Custom|SpawnPlayer
  (params (Controller :type New%20Player%20Controller%20Object%20Reference) (PlayerState :type New%20Player%20State%20Object%20Reference))
  (bind _asfirst_person_gamemode (Utilities|Casting|CastToFirstPersonGamemode (Game|GetGameMode)))
  (Default|SpawnPlayer _asfirst_person_gamemode Controller (Variables|NewPlayerState_C|GetCreateAClass PlayerState)))

(event EventBeginPlay
  (bind (_createaclass _selectedkillstreaks) (CallFunction|LoadPlayerInfo))
  (Variables|Default|SetCreateAClass _createaclass)
  (Variables|Default|SetSelectedKillstreaks _selectedkillstreaks))

(fn ConstructionScript)

(fn OnRepTeam)

(fn OnRepKillstreak)

(fn OnRepMaxHealth)

(fn OnRepHealth)

(fn SavePlayerInfo
  (params (CreateAClass :type Create%20A%20Class%20Structure) (SelectedKillstreaks :type Array%20of%20Killstreak%20Base%20Class%20References))
  (bind _returnvalue (SaveGame|CreateSaveGameObject "/Game/Structs/SaveGameBP.SaveGameBP_C"))
  (bind _output_get (Variables|Default|SetSaveGameRef _returnvalue))
  (Variables|/Game/Structs/SaveGameBP.SaveGameBP_C|SetCreateAClassSave _output_get CreateAClass)
  (Variables|/Game/Structs/SaveGameBP.SaveGameBP_C|SetSelectedKillstreaksSave _output_get SelectedKillstreaks)
  (bind _returnvalue_2 (SaveGame|SaveGametoSlot (Variables|Default|GetSaveGameRef) "CreateAClassSave"))
  (if _returnvalue_2
    (Development|PrintString "saved")
    (else
      (Development|PrintString "error"))))

(fn LoadPlayerInfo
  (bind _returnvalue (SaveGame|DoesSaveGameExist "CreateAClassSave"))
  (if _returnvalue
    (bind _returnvalue_2 (SaveGame|LoadGamefromSlot "CreateAClassSave"))
    (bind _assave_game_bp (Utilities|Casting|CastToSaveGameBP _returnvalue_2))
    (return (Variables|/Game/Structs/SaveGameBP.SaveGameBP_C|GetCreateAClassSave _assave_game_bp) (Variables|/Game/Structs/SaveGameBP.SaveGameBP_C|GetSelectedKillstreaksSave _assave_game_bp))
    (else
      (return "" 0))))