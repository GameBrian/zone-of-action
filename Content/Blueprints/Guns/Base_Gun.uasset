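; Base gun actor for a first-person shooter, providing automatic fire, reloading, recoil and aim-down-sights, with AK47 sounds and animations.
; Looping timers drive FireFunction for ammo, recoil and movement-based spread, and FireClientFunction for montages and muzzle effects.
; FireServer multi-line-traces from the camera, sending hitmarkers and passing character hits to FirstPersonGamemode for damage.
; Recoil accumulates random pitch and yaw kicks, which timed functions then ease back.
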(event Custom|Fire
  (params (OriginalActor :type First%20Person%20Character%20Object%20Reference) (PlayerController :type New%20Player%20Controller%20Object%20Reference) (OriginalPlayerState :type New%20Player%20State%20Object%20Reference))
  ;[1 1 1] Fire
  (Variables|Default|SetOriginalActor OriginalActor)
  (Variables|Default|SetPlayerController PlayerController)
  (CallFunction|FireFunction)
  (Utilities|Time|SetTimerbyFunctionName 0 "FireFunction" (Variables|Default|GetFirerate) true))

(event Custom|PlaySoundForAll
  (params (Location :type Vector))
  ;[1 1 1] Fire
  (Audio|PlaySoundatLocation "/Game/Sound/Guns/Ak47/AK47Shot.AK47Shot" Location))

(event Custom|ReloadOwner
  (params (SkeletalMesh :type Skeletal%20Mesh%20Component%20Object%20Reference))
  ;[1 1 1] Reload
  (Animation|Montage|MontagePlay (Components|SkeletalMesh|GetAnimInstance (Variables|Default|GetGun)) "/Game/Models/Guns/AK47/Weapons/Ark47/Animations/WPANM_FPArms_ArK-47_Reload_Montage.WPANM_FPArms_ArK-47_Reload_Montage" (Variables|Default|GetReloadTime) "MontageLength" 0.0)
  (bind _returnvalue (Animation|Montage|MontagePlay (Components|SkeletalMesh|GetAnimInstance SkeletalMesh) "/Game/Characters/Arms/Animations/CHANM_FPArms_ArK-47_Reload_Montage.CHANM_FPArms_ArK-47_Reload_Montage" 1.0 "MontageLength" 0.0))
  (Variables|Default|SetDelay _returnvalue))

(event Custom|FireClient
  ;[1 1 1] Fire
  (CallFunction|FireClientFunction)
  (Utilities|Time|SetTimerbyFunctionName 0 "FireClientFunction" (Variables|Default|GetFirerate) true))

(event Custom|Recoil
  (params (FirstPersonCharacter :type First%20Person%20Character%20Object%20Reference))
  ;[1 1 1] Recoil
  (Audio|PlaySoundatLocation "/Game/Sound/Guns/Ak47/AK47Shot.AK47Shot" (Transformation|GetActorLocation FirstPersonCharacter))
  (bind _output_get (Variables|Default|SetRecoilPitchVariable (Math|Random|RandomFloatinRange 0.0 -0.1)))
  (Pawn|Input|AddControllerPitchInput FirstPersonCharacter _output_get)
  (bind _output_get_2 (Variables|Default|SetRecoilYawVariable (Math|Random|RandomFloatinRange -0.1 0.1)))
  (Pawn|Input|AddControllerYawInput FirstPersonCharacter _output_get_2)
  (Variables|Default|SetRecoilPitchTotalVariable (+ _output_get (Variables|Default|GetRecoilPitchTotalVariable)))
  (Variables|Default|SetRecoilYawTotalVariable (+ _output_get_2 (Variables|Default|GetRecoilYawTotalVariable)))
  (Utilities|FlowControl|RetriggerableDelay 0.1)
  (Utilities|Time|SetTimerbyFunctionName 0 "RecoilReturn" 0.01 true)
  (Utilities|Time|SetTimerbyFunctionName 0 "RecoilReturnYaw" 0.01 true))

(event Custom|Reload
  (params (SkeletalMesh :type Skeletal%20Mesh%20Component%20Object%20Reference))
  ;[1 1 1] Reload
  (if (< (Variables|Default|GetAmmo) (Variables|Default|GetMaxAmmo))
    (CallFunction|ReloadOwner SkeletalMesh)
    (Variables|Default|SetIsReloading true)
    (Utilities|FlowControl|Delay (Variables|Default|GetDelay))
    (Variables|Default|SetAmmo (Variables|Default|GetMaxAmmo))
    (Variables|Default|SetIsReloading false)))

(event Custom|AimDownSights
  (params (Gun :type Base%20Gun%20Object%20Reference) (FirstPersonCharacter :type First%20Person%20Character%20Object%20Reference))
  ;[1 1 1] ADS
  (Variables|Base_Gun_C|SetAimingDownSights Gun true)
  (Variables|Base_Gun_C|SetMinSpread Gun 0.0)
  (Variables|Base_Gun_C|SetMaxSpread Gun 0.0)
  (Variables|/Script/Engine.CharacterMovementComponent|SetMaxWalkSpeed (Variables|/Script/Engine.Character|GetCharacterMovement FirstPersonCharacter) 3.5e+02))

(event Custom|ReleaseAimDownSights
  (params (Gun :type Base%20Gun%20Object%20Reference) (FirstPersonCharacter :type First%20Person%20Character%20Object%20Reference) (AimingDownSights :type Boolean))
  ;[1 1 1] ADS
  (Variables|Base_Gun_C|SetAimingDownSights Gun AimingDownSights)
  (Variables|Base_Gun_C|SetMinSpread Gun (Variables|Default|GetGunStillMinSpread))
  (Variables|Base_Gun_C|SetMaxSpread Gun (Variables|Default|GetGunStillMaxSpread)))

(event Custom|FireServer
  (params (Start :type Vector) (End :type Vector) (HitBy :type New%20Player%20State%20Object%20Reference) (Impulse :type Vector) (GunRef :type Base%20Gun%20Object%20Reference) (OriginalCharacter :type First%20Person%20Character%20Object%20Reference))
  ;[1 1 1] Fire
  (bind (_outhits _returnvalue) (Collision|MultiLineTraceByChannel Start End "TraceTypeQuery3" true (Utilities|Array|MakeArray OriginalCharacter) "ForDuration" true "(R=1.000000,G=0.000000,B=0.000000,A=1.000000)" "(R=0.000000,G=1.000000,B=0.000000,A=1.000000)" 1e+01))
  (if _returnvalue
    (for _array_element _outhits
      (bind _asfirst_person_character (Utilities|Casting|CastToFirstPersonCharacter (.HitActor (Collision|BreakHitResult _array_element))))
      (bind _asnew_player_state (Utilities|Casting|CastToNewPlayerState (Variables|/Script/Engine.Pawn|GetPlayerState _asfirst_person_character)))
      (Default|Hitmarker HitBy OriginalCharacter)
      (bind _asfirst_person_gamemode (Utilities|Casting|CastToFirstPersonGamemode (Game|GetGameMode)))
      (Default|DamageandCheckifPlayerDead _asfirst_person_gamemode _asfirst_person_character HitBy _asnew_player_state Impulse (.Location (Collision|BreakHitResult _array_element)) self false false (Variables|Default|GetDamage)))))

(event EventBeginPlay
  ;[1 1 1] Fire
)

(event Collision|EventActorBeginOverlap
  (params (OtherActor :type Actor%20Object%20Reference))
  ;[1 1 1] Fire
)

(fn ConstructionScript)

(fn FireFunction
  (bind _originalactor (Variables|Default|GetOriginalActor))
  (bind _originalactor_2 (Variables|Default|GetOriginalActor))
  (bind _firstpersoncamera (Variables|/Game/Blueprints/FPSCharacter/FirstPersonCharacter.FirstPersonCharacter_C|GetFirstPersonCamera _originalactor_2))
  (bind _returnvalue (Transformation|GetWorldLocation _firstpersoncamera))
  (bind _returnvalue_2 (Math|Vector|GetForwardVector _firstpersoncamera))
  (bind (_x _y _z) (Math|Vector|BreakVector _returnvalue_2))
  (CallFunction|CheckAmmo)
  (if (Math|Boolean|ANDBoolean (not (Variables|Default|GetIsReloading)) (Variables|Default|GetHasAmmo) (Variables|/Game/Blueprints/FPSCharacter/FirstPersonCharacter.FirstPersonCharacter_C|GetLMBPressed _originalactor) (not (Variables|/Game/Blueprints/FPSCharacter/FirstPersonCharacter.FirstPersonCharacter_C|GetIsSprinting _originalactor)))
    (CallFunction|DecreaseAmmo)
    (CallFunction|Recoil _originalactor)
    (bind _asnew_player_state (Utilities|Casting|CastToNewPlayerState (Variables|/Script/Engine.Pawn|GetPlayerState (Variables|Default|GetOriginalActor))))
    (if (> (Math|Vector|VectorLength (Transformation|GetVelocity _originalactor)) 0.0)
      (if (Variables|Default|GetAimingDownSights)
        _
        (else
          (Variables|Default|SetMinSpread (Variables|Default|GetGunMovingMinSpread))
          (Variables|Default|SetMaxSpread (Variables|Default|GetGunMovingMaxSpread))))
      (elif (Variables|Default|GetAimingDownSights)
        _
        (else
          (Variables|Default|SetMinSpread (Variables|Default|GetGunStillMinSpread))
          (Variables|Default|SetMaxSpread (Variables|Default|GetGunStillMaxSpread)))))
    (CallFunction|FireServer _returnvalue (+ _returnvalue (* (Math|Vector|MakeVector (+ _x (Math|Random|RandomFloatinRange (Variables|Default|GetMinSpread) (Variables|Default|GetMaxSpread))) (+ _y (Math|Random|RandomFloatinRange (Variables|Default|GetMinSpread) (Variables|Default|GetMaxSpread))) (+ _z (Math|Random|RandomFloatinRange (Variables|Default|GetMinSpread) (Variables|Default|GetMaxSpread)))) 1e+05)) _asnew_player_state (/ (* (Math|Vector|MakeVector (+ _x (Math|Random|RandomFloatinRange (Variables|Default|GetMinSpread) (Variables|Default|GetMaxSpread))) (+ _y (Math|Random|RandomFloatinRange (Variables|Default|GetMinSpread) (Variables|Default|GetMaxSpread))) (+ _z (Math|Random|RandomFloatinRange (Variables|Default|GetMinSpread) (Variables|Default|GetMaxSpread)))) 1e+05) 2.5) self _originalactor)
    (return)
    (else
      (Class|KismetSystemLibrary|PauseTimer 0 "FireFunction"))))

(fn RecoilReturn
  (if (> (Math|Float|Absolute(Float) (Variables|Default|GetRecoilPitchTotalVariable)) 0.08)
    (Pawn|Input|AddControllerPitchInput (Variables|Default|GetOriginalActor) 0.08)
    (Variables|Default|SetRecoilPitchTotalVariable (- (Math|Float|Absolute(Float) (Variables|Default|GetRecoilPitchTotalVariable)) 0.08))
    (else
      (Pawn|Input|AddControllerPitchInput (Variables|Default|GetOriginalActor) (Math|Float|Absolute(Float) (Variables|Default|GetRecoilPitchTotalVariable)))
      (Variables|Default|SetRecoilPitchTotalVariable 0.0)
      (Class|KismetSystemLibrary|PauseTimer 0 "RecoilReturn"))))

(fn RecoilReturnYaw
  (if (or (> (Variables|Default|GetRecoilYawTotalVariable) 0.08) (< (Variables|Default|GetRecoilYawTotalVariable) -0.08))
    (if (> (Variables|Default|GetRecoilYawTotalVariable) 0.0)
      (Pawn|Input|AddControllerYawInput (Variables|Default|GetOriginalActor) -0.08)
      (Variables|Default|SetRecoilYawTotalVariable (+ (Variables|Default|GetRecoilYawTotalVariable) -0.08))
      (else
        (Pawn|Input|AddControllerYawInput (Variables|Default|GetOriginalActor) 0.08)
        (Variables|Default|SetRecoilYawTotalVariable (+ (Variables|Default|GetRecoilYawTotalVariable) 0.08))))
    (else
      (Pawn|Input|AddControllerYawInput (Variables|Default|GetOriginalActor) (Variables|Default|GetRecoilYawTotalVariable))
      (Variables|Default|SetRecoilYawVariable 0.0)
      (Class|KismetSystemLibrary|PauseTimer 0 "RecoilReturnYaw"))))

(fn CheckAmmo
  (if (> (Variables|Default|GetAmmo) 0)
    (Variables|Default|SetHasAmmo true)
    (else
      (Variables|Default|SetHasAmmo false))))

(fn FireClientFunction
  (bind _originalactor (Variables|Default|GetOriginalActor))
  (if (Math|Boolean|ANDBoolean (not (Variables|Default|GetIsReloading)) (Variables|Default|GetHasAmmo) (Variables|/Game/Blueprints/FPSCharacter/FirstPersonCharacter.FirstPersonCharacter_C|GetLMBPressedClient _originalactor) (not (Variables|/Game/Blueprints/FPSCharacter/FirstPersonCharacter.FirstPersonCharacter_C|GetIsSprinting _originalactor)))
    (if (Variables|Default|GetAimingDownSights)
      (Animation|Montage|MontagePlay (Components|SkeletalMesh|GetAnimInstance (Variables|/Game/Blueprints/FPSCharacter/FirstPersonCharacter.FirstPersonCharacter_C|GetArms (Variables|Default|GetOriginalActor))) "/Game/Characters/Arms/Animations/CHANM_FPArms_ArK-47_ADS-Fire_Montage.CHANM_FPArms_ArK-47_ADS-Fire_Montage" 2.0 "MontageLength" 0.0)
      (Animation|Montage|MontagePlay (Components|SkeletalMesh|GetAnimInstance (Variables|Default|GetGun)) "/Game/Models/Guns/AK47/Weapons/Ark47/Animations/WPANM_FPArms_ArK-47_Fire_Montage.WPANM_FPArms_ArK-47_Fire_Montage" 2.0 "MontageLength" 0.0)
      (Effects|SpawnEmitterAttached "/Game/Models/Guns/AK47/Particles/PS_VFX_ArK47.PS_VFX_ArK47" (Variables|Default|GetGun) "Fire_FX_Slot")
      (else
        (Animation|Montage|MontagePlay (Components|SkeletalMesh|GetAnimInstance (Variables|/Game/Blueprints/FPSCharacter/FirstPersonCharacter.FirstPersonCharacter_C|GetArms (Variables|Default|GetOriginalActor))) "/Game/Characters/Arms/Animations/CHANM_FPArms_ArK-47_Fire_Montage.CHANM_FPArms_ArK-47_Fire_Montage" 2.0 "MontageLength" 0.0)
        (Animation|Montage|MontagePlay (Components|SkeletalMesh|GetAnimInstance (Variables|Default|GetGun)) "/Game/Models/Guns/AK47/Weapons/Ark47/Animations/WPANM_FPArms_ArK-47_Fire_Montage.WPANM_FPArms_ArK-47_Fire_Montage" 2.0 "MontageLength" 0.0)
        (Effects|SpawnEmitterAttached "/Game/Models/Guns/AK47/Particles/PS_VFX_ArK47.PS_VFX_ArK47" (Variables|Default|GetGun) "Fire_FX_Slot")))
    (else
      (Class|KismetSystemLibrary|PauseTimer 0 "FireClientFunction"))))

(fn ReloadonOwner
  (params (SkeletalMesh :type Skeletal%20Mesh%20Component%20Object%20Reference))
  (Animation|Montage|MontagePlay (Components|SkeletalMesh|GetAnimInstance (Variables|Default|GetGun)) "/Game/Models/Guns/AK47/Weapons/Ark47/Animations/WPANM_FPArms_ArK-47_Reload_Montage.WPANM_FPArms_ArK-47_Reload_Montage" (Variables|Default|GetReloadTime) "MontageLength" 0.0)
  (bind _returnvalue (Animation|Montage|MontagePlay (Components|SkeletalMesh|GetAnimInstance SkeletalMesh) "/Game/Characters/Arms/Animations/CHANM_FPArms_ArK-47_Reload_Montage.CHANM_FPArms_ArK-47_Reload_Montage" 1.0 "MontageLength" 0.0))
  (return _returnvalue))

(fn DecreaseAmmo
  (Variables|Default|SetAmmo (- (Variables|Default|GetAmmo) 1)))