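; Grenade lethal that damages player characters within a radius when its countdown ends.
; BeginPlay starts a looping one-second timer that decrements TimeLeft, then calls Blowup and pauses itself at zero.
; Blowup runs a debug-drawn multi-sphere trace, passing each character hit to FirstPersonGamemode's DamageAndCheckIfPlayerDead with fixed damage and the Instigator's player state.
; The KilledSelf flag is set true when the victim is not the Instigator, opposite to its name.
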(event Custom|StartCountdown
  (Utilities|Time|SetTimerbyFunctionName 0 "GrenadeTimer" 1.0 true))

(event Custom|Blowup
  (bind _returnvalue (Transformation|GetActorLocation))
  (bind (_outhits _returnvalue_2) (Collision|MultiSphereTraceByChannel _returnvalue _returnvalue 3.5e+02 "TraceTypeQuery3" true 0 "ForDuration"))
  (if _returnvalue_2
    (for _array_element _outhits
      (bind _asfirst_person_character (Utilities|Casting|CastToFirstPersonCharacter (.HitActor (Collision|BreakHitResult _array_element))))
      (bind _asnew_player_state (Utilities|Casting|CastToNewPlayerState (Variables|/Script/Engine.Pawn|GetPlayerState _asfirst_person_character)))
      (bind _asnew_player_state_2 (Utilities|Casting|CastToNewPlayerState (Variables|/Script/Engine.Pawn|GetPlayerState (Variables|Default|GetInstigator))))
      (bind _asfirst_person_gamemode (Utilities|Casting|CastToFirstPersonGamemode (Game|GetGameMode)))
      (Default|DamageandCheckifPlayerDead _asfirst_person_gamemode _asfirst_person_character _asnew_player_state_2 _asnew_player_state "0, 0, 0" (.Location (Collision|BreakHitResult _array_element)) 0 (not (== _asfirst_person_character (Variables|Default|GetInstigator))) true 1e+02))))

(event EventBeginPlay
  (CallFunction|StartCountdown))

(fn ConstructionScript
  (|CallParentFunction))

(fn GrenadeTimer
  (bind _output_get (Variables|Default|SetTimeLeft (- (Variables|Default|GetTimeLeft) 1)))
  (if (<= _output_get 0)
    (CallFunction|Blowup)
    (Class|KismetSystemLibrary|PauseTimer 0 "GrenadeTimer")))